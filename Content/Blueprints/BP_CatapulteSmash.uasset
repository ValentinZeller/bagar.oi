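; Catapult hazard or launcher for the Smash mode that flings any BP_PaperPlayer hitting its box.
; On hit it applies a velocity-change impulse built from the actor's forward vector scaled by a horizontal force, plus a vertical force.
; If that player has no life points left and the game is unfinished, it calls Scoring on BP_GameModeSmash through a DoOnce that resets right afterward.
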(event OnComponentHit(Box)
  (params (HitComponent :type Primitive%20Component%20Object%20Reference) (OtherActor :type Actor%20Object%20Reference) (OtherComp :type Primitive%20Component%20Object%20Reference) (NormalImpulse :type Vector :default "0, 0, 0") (Hit :type Hit%20Result%20Structure%20%28by%20ref%29))
  (bind _asbp_paper_player (Utilities|Casting|CastToBP_PaperPlayer OtherActor))
  (Physics|AddImpulse (Variables|/Script/Engine.Character|GetCharacterMovement _asbp_paper_player) (+ (* (Transformation|GetActorForwardVector) (Variables|Default|GetHorizontalForce)) (Variables|Default|GetVerticalAddForce)) true)
  (if (<= (Variables|/Game/Blueprints/BP_PaperPlayer.BP_PaperPlayer_C|GetCurrentLifePoints _asbp_paper_player) 0.0)
    (bind _asbp_game_mode_smash (Utilities|Casting|CastToBP_GameModeSmash (Game|GetGameMode)))
    (if (not (Variables|/Game/Blueprints/BP_GameModeSmash.BP_GameModeSmash_C|GetIsGameFinished _asbp_game_mode_smash))
      (Utilities|FlowControl|DoOnce false :!label _label
        (:Completed
          (Default|Scoring _asbp_game_mode_smash _asbp_paper_player)
          (goto _label Reset))))))

(event EventBeginPlay)

(event Collision|EventActorBeginOverlap
  (params (OtherActor :type Actor%20Object%20Reference)))

(event EventTick
  (params (DeltaSeconds :type Float%20%28single-precision%29)))

(fn ConstructionScript)