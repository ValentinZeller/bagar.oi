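; Game mode for a two-player local versus game with Paper2D characters, handling spawning, scoring and match end.
; On BeginPlay it matches PlayerStart tags to player indices, creates extra local players, then spawns and possesses a BP_PaperPlayer for each.
; Scoring awards the opponent a point, then revives the given player in place with full life and a reversed flipbook.
; Tick flags the game finished once either score reaches the maximum.
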(event EventBeginPlay
  (CallFunction|GetPlayerStartPoints)
  (CallFunction|SpawnPlayers))

(event EventTick
  (params (DeltaSeconds :type Float%20%28single-precision%29))
  (if (or (>= (Variables|Default|GetP1score) (Variables|Default|GetScoreMax)) (>= (Variables|Default|GetP2score) (Variables|Default|GetScoreMax)))
    (Utilities|FlowControl|DoOnce false
      (:Completed
        (Variables|Default|SetIsGameFinished true)))))

(fn ConstructionScript)

(fn GetPlayerStartPoints
  (bind _outactors (Actor|GetAllActorsOfClass "/Script/Engine.PlayerStart"))
  (Variables|Default|SetPlayerStartArray _outactors))

(fn SpawnPlayers
  (for _index (range 0 (- (Variables|Default|GetMaxPlayer) 1))
    (Variables|Default|SetIndex _index)
    (for _array_element (Variables|Default|GetPlayerStartArray)
      (if (Utilities|Name|Equal(Name) (Variables|/Script/Engine.PlayerStart|GetPlayerStartTag _array_element) (Utilities|String|StringToName (Utilities|String|ToString(Integer) (Variables|Default|GetIndex))))
        (if (== (Variables|Default|GetIndex) 0)
          _
          (else
            (Class|GameplayStatics|CreatePlayer (Variables|Default|GetIndex))))
        (bind _returnvalue (Game|SpawnActorfromClass "/Game/Blueprints/BP_PaperPlayer.BP_PaperPlayer_C" (Transformation|GetActorTransform _array_element) "Undefined" 0 0))
        (if (== (Variables|Default|GetIndex) 1)
          (Variables|/Game/Blueprints/BP_PaperPlayer.BP_PaperPlayer_C|SetPlayerNumber _returnvalue 1))
        (Pawn|Possess (Game|GetPlayerController (Variables|Default|GetIndex)) _returnvalue)
        (Utilities|Array|AddUnique (Variables|Default|GetPlayers) _returnvalue)))))

(fn Scoring
  (params (Player :type BP%20Paper%20Player%20Object%20Reference))
  (LocalVariables|SetPlayerTargeted Player)
  (if (== Player (Utilities|Array|Get(acopy) (Variables|Default|GetPlayers)))
    (Math|Integer|IncrementInt (Variables|Default|GetP2score)
      (:%20%20
        _))
    (else
      (Math|Integer|IncrementInt (Variables|Default|GetP1score)
        (:%20%20
          _))))
  (Variables|/Game/Blueprints/BP_PaperPlayer.BP_PaperPlayer_C|SetCurrentLifePoints (LocalVariables|GetPlayerTargeted) (Variables|/Game/Blueprints/BP_PaperPlayer.BP_PaperPlayer_C|GetMaxLifePoints (LocalVariables|GetPlayerTargeted)))
  (Components|Timeline|ReversefromEnd (Variables|/Script/Paper2D.PaperCharacter|GetSprite (LocalVariables|GetPlayerTargeted)))
  (Audio|Components|Audio|Play (Variables|/Script/Paper2D.PaperCharacter|GetSprite (LocalVariables|GetPlayerTargeted)))
  (Variables|/Game/Blueprints/BP_PaperPlayer.BP_PaperPlayer_C|SetbIsDead (LocalVariables|GetPlayerTargeted) false))