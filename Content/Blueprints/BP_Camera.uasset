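; BP_Camera is a shared camera actor that becomes the view target for every player controller when play begins.
; On BeginPlay, ClassSetup caches BP_GameMode and its Players array, then calls SetViewTargetWithBlend on all PlayerControllers to point them at itself.
; It stores the first two Players entries as P1 and P2, though this Blueprint has no Tick logic that uses them.
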(event EventBeginPlay
  (CallFunction|ClassSetup))

(event Collision|EventActorBeginOverlap
  (params (OtherActor :type Actor%20Object%20Reference)))

(event EventTick
  (params (DeltaSeconds :type Float%20%28single-precision%29)))

(fn ConstructionScript)

(fn ClassSetup
  (bind _asbp_game_mode (Utilities|Casting|CastToBP_GameMode (Game|GetGameMode)))
  (bind _output_get (Variables|Default|SetBP_GameMode _asbp_game_mode))
  (Variables|Default|SetPlayers (Variables|/Game/Blueprints/BP_GameMode.BP_GameMode_C|GetPlayers _output_get))
  (bind _outactors (Actor|GetAllActorsOfClass "/Script/Engine.PlayerController"))
  (Game|Player|SetViewTargetwithBlend _outactors self 0.0 "VTBlend_Linear" 0.0 false)
  (for (_array_element _array_index) (Variables|Default|GetPlayers)
    (switch int _array_index
      (:0
        (Variables|Default|SetP1 _array_element))
      (:1
        (Variables|Default|SetP2 _array_element)))))